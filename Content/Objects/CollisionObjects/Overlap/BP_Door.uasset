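; BP_Door is an interactable door that opens for a character and closes itself on a timer.
; Overlap by a BP_ThirdPersonCharacter sends it a StartInteract message.
; StartInteract, if the door is closed, rotates the Door component via GetOpenDoorRotator, then schedules CloseDoor to reset it to zero rotation after a short delay.
; GetOpenDoorRotator's facing-based yaw calculation is left unconnected.
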(event Custom|OnCloseDoor
  (CallFunction|CloseDoor))

(event Collision|EventActorBeginOverlap
  (params (OtherActor :type Actor%20Object%20Reference))
  (bind _asbp_third_person_character (Utilities|Casting|CastToBP_ThirdPersonCharacter OtherActor))
  (Class|BPIInteractable|StartInteract(Message) self _asbp_third_person_character))

(event EventStartInteract
  (params (Character :type BP%20Third%20Person%20Character%20Object%20Reference))
  (if (CallFunction|IsClosed)
    (CallFunction|OpenDoor Character)
    (Utilities|Time|SetTimerbyEvent (delegate Custom|OnCloseDoor) 2.0 false 2.0)))

(fn ConstructionScript)

(fn OpenDoor
  (params (Character :type BP%20Third%20Person%20Character%20Object%20Reference))
  (Transformation|SetRelativeRotation (Variables|Default|GetDoor) (Utilities|GetOpenDoorRotator Character) false false))

(fn CloseDoor
  (Transformation|SetRelativeRotation (Variables|Default|GetDoor) "0, 0, 0" false false))

(fn IsClosed
  (return (Utilities|Operators|EqualEqual :A (Variables|/Script/Engine.SceneComponent|GetRelativeRotation (Variables|Default|GetDoor)))))

(fn Name
  (return "None"))