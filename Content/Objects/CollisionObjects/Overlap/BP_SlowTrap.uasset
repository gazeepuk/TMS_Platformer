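; BP_SlowTrap is an overlap trap that slows a BP_ThirdPersonCharacter while it stands inside.
; Begin overlap calls the OnBeginOverlap function, which halves the character's current max walk speed.
; End overlap doubles the current speed inline rather than calling OnEndOverlap.
; OnEndOverlap does the same doubling, but reads the speed from OverlapedCharacter instead of its Character argument, then calls the parent.
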(event Collision|EventActorBeginOverlap
  (params (OtherActor :type Actor%20Object%20Reference))
  (bind _asbp_third_person_character (Utilities|Casting|CastToBP_ThirdPersonCharacter OtherActor))
  (CallFunction|OnBeginOverlap _asbp_third_person_character))

(event Collision|EventActorEndOverlap
  (params (OtherActor :type Actor%20Object%20Reference))
  (bind _asbp_third_person_character (Utilities|Casting|CastToBP_ThirdPersonCharacter OtherActor))
  (Default|SetMaxWalkSpeed _asbp_third_person_character (* (Default|GetCurrentMaxWalkSpeed _asbp_third_person_character) 2.0)))

(fn ConstructionScript
  (|CallParentFunction))

(fn OnBeginOverlap
  (params (Character :type BP%20Third%20Person%20Character%20Object%20Reference))
  (Default|SetMaxWalkSpeed Character (* (Default|GetCurrentMaxWalkSpeed Character) 0.5)))

(fn OnEndOverlap
  (params (Character :type BP%20Third%20Person%20Character%20Object%20Reference))
  (Default|SetMaxWalkSpeed Character (* (Default|GetCurrentMaxWalkSpeed (Variables|Default|GetOverlapedCharacter)) 2.0))
  (|CallParentFunction Character))