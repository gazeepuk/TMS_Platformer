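; BP_EffectObject is a pickup that applies an effect to the character that overlaps it, then destroys itself.
; Its construction script instantiates an Effect object from EffectClass.
; The OnBeginOverlap override calls the parent, then starts the effect's impact, passing the character and EffectInfo, so the effect's behavior lives in the effect class rather than the pickup.
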(event EventBeginPlay)

(event Collision|EventActorBeginOverlap
  (params (OtherActor :type Actor%20Object%20Reference))
  (|CallParentFunction OtherActor) ; This node is disabled and will not be called.\nDrag off pins to build functionality.
)

(event EventTick
  (params (DeltaSeconds :type Float%20%28single-precision%29)))

(fn ConstructionScript
  (|CallParentFunction)
  (bind _returnvalue (Game|ConstructObjectfromClass (Variables|Default|GetEffectClass)))
  (Variables|Default|SetEffect _returnvalue))

(fn OnBeginOverlap
  (params (Character :type BP%20Third%20Person%20Character%20Object%20Reference))
  (|CallParentFunction Character)
  (Default|EventBeginEffectImpact (Variables|Default|GetEffect) Character (Variables|Default|GetEffectInfo))
  (Actor|DestroyActor))