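; BP_DamageOverlap is an overlap-triggered actor that damages a character with a BP_StatsComponent, then destroys itself.
; OnBeginOverlap calls the parent handler, then BlowUp, which applies Damage through GetDamage on the OverlapedCharacter's stats component.
; An unconnected TODO branch sketches a radius sphere trace that would damage nearby actors and chain BlowUp into other BP_DamageOverlap actors.
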(fn ConstructionScript)

(fn OnBeginOverlap
  (params (Character :type BP%20Third%20Person%20Character%20Object%20Reference))
  (|CallParentFunction Character)
  (Utilities|IsValid (Actor|GetComponentbyClass Character "/Game/Characters/ThirdPerson/Blueprints/Components/BP_StatsComponent.BP_StatsComponent_C")
    (:Is%20Valid
      (CallFunction|BlowUp))))

(fn BlowUp
  (bind _overlapedcharacter (Variables|Default|GetOverlapedCharacter))
  (bind _returnvalue (Actor|GetComponentbyClass _overlapedcharacter "/Game/Characters/ThirdPerson/Blueprints/Components/BP_StatsComponent.BP_StatsComponent_C"))
  (Utilities|IsValid _returnvalue
    (:Is%20Valid
      (Default|GetDamage _returnvalue (Variables|Default|GetDamage))
      (Actor|DestroyActor))))