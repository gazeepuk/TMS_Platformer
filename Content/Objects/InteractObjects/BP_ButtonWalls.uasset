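; BP_ButtonWalls is an interactable button that switches the visibility of an assigned set of walls.
; A text prompt is shown while the third-person character overlaps the actor and hidden when it leaves.
; The Interact event calls SwitchWalls, which loops over the Walls array and calls SwitchVisibility on each element.
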(event EventBeginPlay)

(event Collision|EventActorBeginOverlap
  (params (OtherActor :type Actor%20Object%20Reference))
  (Utilities|Casting|CastToBP_ThirdPersonCharacter OtherActor)
  (Development|SetHiddeninGame (Variables|Default|GetTextRender) false false))

(event Collision|EventActorEndOverlap
  (params (OtherActor :type Actor%20Object%20Reference))
  (Utilities|Casting|CastToBP_ThirdPersonCharacter OtherActor)
  (Development|SetHiddeninGame (Variables|Default|GetTextRender) true false))

(event EventInteract
  (params (Character :type BP%20Third%20Person%20Character%20Object%20Reference))
  (CallFunction|SwitchWalls))

(fn ConstructionScript)

(fn SwitchWalls
  (for _array_element (Variables|Default|GetWalls)
    (CallFunction|SwitchVisibility _array_element)))