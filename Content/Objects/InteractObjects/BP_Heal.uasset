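; Interactable object Blueprint that heals a character when used.
; Impact reveals the InteractText prompt, and ending an actor overlap hides it again.
; Interact calls Heal on the passed Character for a fixed amount, with no use limit or self-removal in this graph.
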(event Collision|EventActorBeginOverlap
  (params (OtherActor :type Actor%20Object%20Reference))
  (|CallParentFunction OtherActor) ; This node is disabled and will not be called.\nDrag off pins to build functionality.
)

(event EventInteract
  (params (Character :type BP%20Third%20Person%20Character%20Object%20Reference))
  (Default|Heal Character 1))

(event Collision|EventActorEndOverlap
  (params (OtherActor :type Actor%20Object%20Reference))
  (Development|SetHiddeninGame (Variables|Default|GetInteractText) true false))

(fn ConstructionScript
  (|CallParentFunction))

(fn Impact
  (params (Character :type BP%20Third%20Person%20Character%20Object%20Reference))
  (Development|SetHiddeninGame (Variables|Default|GetInteractText) false false))