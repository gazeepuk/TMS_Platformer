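; BP_StateMachine is a state machine component that drives the behavior of BP_ThirdPersonCharacter.
; On BeginPlay it casts its owner to that character and caches the reference.
; SetState exits the current state object if valid, constructs a new one from the given class with the character as outer, then calls Enter on it with the character.
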(event EventBeginPlay
  (bind _asbp_third_person_character (Utilities|Casting|CastToBP_ThirdPersonCharacter (Components|GetOwner)))
  (Variables|Default|SetCharacter _asbp_third_person_character))

(fn SetState
  (params (State :type BP%20Character%20State%20Base%20Class%20Reference))
  (Utilities|IsValid (Variables|Default|GetCurrentState)
    (:Is%20Valid
      (Default|Exit (Variables|Default|GetCurrentState)))
    (:Is%20Not%20Valid
      _))
  (bind _returnvalue (Game|ConstructObjectfromClass (Variables|Default|GetCharacter) State))
  (bind _output_get (Variables|Default|SetCurrentState _returnvalue))
  (Default|Enter _output_get (Variables|Default|GetCharacter)))