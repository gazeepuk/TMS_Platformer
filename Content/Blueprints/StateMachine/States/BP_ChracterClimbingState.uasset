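; Character state for climbing, part of the character state machine.
; On enter it switches movement to Flying and makes the character follow controller yaw.
; Movement input moves the character along its right and up vectors, so it travels across a vertical plane.
; Starting a jump launches the character, stopping calls StopJumping, and rotation input is ignored.
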(fn AddMovement
  (params (Value%20X :type Float%20%28double-precision%29) (Value%20Y :type Float%20%28double-precision%29))
  (bind _character (Variables|Default|GetCharacter))
  (bind _returnvalue (Transformation|GetActorRotation _character))
  (Pawn|Input|AddMovementInput _character (Math|Vector|GetRightVector _returnvalue) Value%20X false)
  (Pawn|Input|AddMovementInput _character (Math|Vector|GetUpVector _returnvalue) Value%20Y false))

(fn StartJump
  (Default|Launch (Variables|Default|GetCharacter)))

(fn StopJump
  (Character|StopJumping (Variables|Default|GetCharacter)))

(fn Enter
  (params (Character :type BP%20Third%20Person%20Character%20Object%20Reference))
  (|CallParentFunction Character)
  (Variables|/Script/Engine.Pawn|SetbUseControllerRotationYaw (Variables|Default|GetCharacter) true)
  (Pawn|Components|CharacterMovement|SetMovementMode (Variables|/Script/Engine.Character|GetCharacterMovement (Variables|Default|GetCharacter)) "MOVE_Flying" 0))

(fn AddRotation
  (params (Value%20X :type Float%20%28double-precision%29) (Value%20Y :type Float%20%28double-precision%29)))