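; Walking state for the character state machine, handling movement, look, jump and dash for the owning Character.
; Movement input follows the control rotation's yaw, with roll also applied to the right vector, while look input drives controller yaw and pitch.
; Jump start calls the character's own Launch, and stop calls StopJumping.
; Dash checks StatsComponent stamina, halts movement, launches along actor forward, then spends the cost.
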(fn Enter
  (params (Character :type BP%20Third%20Person%20Character%20Object%20Reference))
  (|CallParentFunction Character))

(fn AddMovement
  (params (Value%20X :type Float%20%28double-precision%29) (Value%20Y :type Float%20%28double-precision%29))
  (bind _character (Variables|Default|GetCharacter))
  (bind _character_2 (Variables|Default|GetCharacter))
  (bind _returnvalue (Pawn|GetControlRotation _character :!class /Script/Engine.Pawn))
  (Pawn|Input|AddMovementInput _character_2 (Math|Vector|GetRightVector (Math|Rotator|MakeRotator (.roll _returnvalue) 0.0 (.yaw _returnvalue))) Value%20X false)
  (Pawn|Input|AddMovementInput _character_2 (Math|Vector|GetForwardVector (Math|Rotator|MakeRotator 0.0 0.0 (.yaw (Pawn|GetControlRotation _character_2 :!class /Script/Engine.Pawn)))) Value%20Y false))

(fn AddRotation
  (params (Value%20X :type Float%20%28double-precision%29) (Value%20Y :type Float%20%28double-precision%29))
  (bind _character (Variables|Default|GetCharacter))
  (Pawn|Input|AddControllerYawInput _character Value%20X)
  (Pawn|Input|AddControllerPitchInput _character Value%20Y))

(fn StartJump
  (Default|Launch (Variables|Default|GetCharacter)))

(fn StopJump
  (Character|StopJumping (Variables|Default|GetCharacter)))

(fn Dash
  (bind _character (Variables|Default|GetCharacter))
  (bind _character_2 (Variables|Default|GetCharacter))
  (bind _character_3 (Variables|Default|GetCharacter))
  (bind _statscomponent (Variables|/Game/Characters/ThirdPerson/Blueprints/BP_ThirdPersonCharacter.BP_ThirdPersonCharacter_C|GetStatsComponent _character_2))
  (if (> (Default|GetCurrentStamina _statscomponent) (Default|GetDashStaminaCost _statscomponent))
    (Components|Movement|StopMovementImmediately (Variables|/Script/Engine.Character|GetCharacterMovement _character))
    (Character|LaunchCharacter _character_3 (* (Math|Vector|GetForwardVector (Transformation|GetActorRotation _character)) 1.5e+03) false false)
    (Default|SpendStamina (Variables|/Game/Characters/ThirdPerson/Blueprints/BP_ThirdPersonCharacter.BP_ThirdPersonCharacter_C|GetStatsComponent _character_3) (Default|GetDashStaminaCost (Variables|/Game/Characters/ThirdPerson/Blueprints/BP_ThirdPersonCharacter.BP_ThirdPersonCharacter_C|GetStatsComponent (Variables|Default|GetCharacter))))))