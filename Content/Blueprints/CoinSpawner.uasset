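; Coin spawner actor that places CoinClass actors at random points inside its Box volume and tracks them in CoinsPool.
; BeginPlay spawns the initial CoinsAmount coins, setting a looping SpawnCoinRate timer within that same loop.
; SpawnCoinsLoop, the apparent timer callback, replaces the first invalid pool entry with a new coin.
; If none is invalid, it appends another coin and sets CoinsAmount to the added index, so the pool can grow.
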(event EventBeginPlay
  (for _index (range 0 (Variables|Default|GetCoinsAmount))
    (bind _returnvalue (CallFunction|SpawnCoin))
    (Utilities|Array|Add (Variables|Default|GetCoinsPool) _returnvalue)
    (Utilities|Time|SetTimerbyEvent (EventDispatchers|CreateEvent :!event SpawnCoinsLoop) (Math|Conversions|ToFloat(Integer) (Variables|Default|GetSpawnCoinRate)) true)))

(fn ConstructionScript)

(fn SpawnCoin
  (bind _box (Variables|Default|GetBox))
  (Game|SpawnActorfromClass (Variables|Default|GetCoinClass) (Math|Transform|MakeTransform (Math|Random|RandomPointinBoundingBox (Transformation|GetWorldLocation _box) (Variables|/Script/Engine.BoxComponent|GetBoxExtent _box)) "0, 0, 0" "1.000000,1.000000,1.000000") "Undefined" "MultiplyWithRoot" 0 0)
  (return 0))

(fn SpawnCoinsLoop
  (bind _coinspool (Variables|Default|GetCoinsPool))
  (bind _index (Utilities|FlowControl|ForLoopwithBreak 0 (Variables|Default|GetCoinsAmount))
    (:LoopBody
      (Utilities|IsValid (Utilities|Array|Get(acopy) _coinspool _index)
        (:Is%20Not%20Valid
          (bind _returnvalue (CallFunction|SpawnCoin))
          (Utilities|Array|SetArrayElem _coinspool _index _returnvalue)
          (return))))
    (:Completed
      (bind _returnvalue_2 (CallFunction|SpawnCoin))
      (bind _returnvalue_3 (Utilities|Array|Add _coinspool _returnvalue_2))
      (Variables|Default|SetCoinsAmount _returnvalue_3)
      (return))))