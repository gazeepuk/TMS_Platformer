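; Health pickup actor that heals an overlapping actor and respawns after a delay.
; On overlap it gets the actor's HealthComponent and, if health is not full, calls TryHeal with its heal amount.
; It then hides its root and children and disables box collision until a one-shot timer restores both.
; The component lookup result is used without a validity check.
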(event Custom|Respawn
  (Development|SetHiddeninGame (Variables|Default|GetDefaultSceneRoot) false true)
  (Collision|SetCollisionEnabled (Variables|Default|GetBox) "QueryOnly"))

(event EventBeginPlay)

(event Collision|EventActorBeginOverlap
  (params (OtherActor :type Actor%20Object%20Reference))
  (bind _output_get (Variables|Default|SetHealthComponent (Actor|GetComponentbyClass OtherActor "/Script/TMS_Platformer.HealthComponent")))
  (if (not (Class|HealthComponent|IsHealthFull _output_get))
    (Class|HealthComponent|TryHeal _output_get (Variables|Default|GetHeal%20Amount))
    (Development|SetHiddeninGame (Variables|Default|GetDefaultSceneRoot) true true)
    (Collision|SetCollisionEnabled (Variables|Default|GetBox) "NoCollision")
    (Utilities|Time|SetTimerbyEvent (delegate Custom|Respawn) (Variables|Default|GetRespawnSpan))))

(event EventTick
  (params (DeltaSeconds :type Float%20%28single-precision%29)))

(fn ConstructionScript)