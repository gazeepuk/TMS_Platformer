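; BP_HealEffect is a character effect that heals its target over its iterations.
; It overrides the first, middle and last iteration hooks, calling the parent version of each before healing.
; A shared HealCharacter function passes the effect value, truncated to an integer, to the character's Heal function.
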(fn FirstIteration
  (|CallParentFunction)
  (CallFunction|HealCharacter))

(fn HealCharacter
  (Default|Heal (Variables|Default|GetCharacter) (Math|Float|Truncate (Variables|Default|GetEffectValue))))

(fn LastIteration
  (|CallParentFunction)
  (CallFunction|HealCharacter))

(fn MiddleIteration
  (|CallParentFunction)
  (CallFunction|HealCharacter))