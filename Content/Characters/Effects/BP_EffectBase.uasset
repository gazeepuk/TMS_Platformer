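; BP_EffectBase is a base Blueprint for timed, tick-based effects on a character.
; On impact it copies value, tick count and duration from the effect info, then spreads ticks evenly across the duration with a looping timer.
; Ticks route to First, Middle and Last iteration functions, which here only print debug text.
; When finished, it clears the timer and removes itself from the character's BP_EffectComponent.
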(event Custom|EventBeginEffectImpact
  (params (CharacterRef :type BP%20Third%20Person%20Character%20Object%20Reference%20%28by%20ref%29) (InEffectInfo :type S%20Effect%20Info%20Structure))
  (CallFunction|InitVariables CharacterRef InEffectInfo)
  (if (> (Variables|Default|GetTicksAmount) 0)
    (CallFunction|FirstIteration)
    (bind _output_get (Variables|Default|SetTicksPassedCount 1))
    (if (< _output_get (Variables|Default|GetTicksAmount))
      (Utilities|Time|SetTimerbyFunctionName 0 "LoopIteration" (Variables|Default|GetCooldown) true)
      (else
        (CallFunction|ClearEffect)))))

(fn InitVariables
  (params (CharacterRef :type BP%20Third%20Person%20Character%20Object%20Reference%20%28by%20ref%29) (InEffectInfo :type S%20Effect%20Info%20Structure))
  (bind (_ticksamount _duration _effectvalue) (Utilities|Struct|BreakS_EffectInfo InEffectInfo))
  (Variables|Default|SetCharacter CharacterRef)
  (Variables|Default|SetEffectValue _effectvalue)
  (bind _output_get (Variables|Default|SetTicksAmount _ticksamount))
  (bind _output_get_2 (Variables|Default|SetDuration _duration))
  ;[1 1 1] Calculate Cooldown
  (Variables|Default|SetCooldown (/ _output_get_2 (- _output_get 1))))

(fn FirstIteration
  (Development|PrintString 0 "First Iteration"))

(fn LastIteration
  (Development|PrintString 0 "Last Iteration"))

(fn MiddleIteration
  (Development|PrintString 0 "Middle Iteration"))

(fn LoopIteration
  (bind _tickspassedcount (Variables|Default|GetTicksPassedCount))
  (bind _returnvalue (+ _tickspassedcount 1))
  ;[1 1 1] (TicksCount < 1 && TicksCount < TicksAmount) => MiddleInteraction
  (if (and (> _returnvalue 1) (< _returnvalue (Variables|Default|GetTicksAmount)))
    (CallFunction|MiddleIteration)
    (Math|Integer|IncrementInt (Variables|Default|GetTicksPassedCount))
    (else
      ;[1 1 1] Clear LoopIteraction
      (if (== (+ (Variables|Default|GetTicksPassedCount) 1) (Variables|Default|GetTicksAmount))
        (Utilities|Time|ClearTimerbyFunctionName 0 "LoopIteration")
        ;[1 1 1] Last Iteraction
        (CallFunction|LastIteration)
        (CallFunction|ClearEffect)
        (else
          (Development|PrintString 0 "EFFECT LOOP ERROR" true true "(R=1.000000,G=0.000000,B=0.076232,A=1.000000)" 5.0))))))

(fn ClearEffect
  (Utilities|Time|ClearTimerbyFunctionName 0 "LoopIteration")
  (Default|RemoveEffect (Actor|GetComponentbyClass (Variables|Default|GetCharacter) "/Game/Characters/Effects/BP_EffectComponent.BP_EffectComponent_C") self)
  (Development|PrintString 0 (Utilities|String|Append "Cleared: " (Utilities|GetDisplayName self))))