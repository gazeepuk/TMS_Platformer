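; BP_PoisonEffect is a character effect that deals poison damage over a series of iterations.
; It extends the parent effect's first, middle and last iteration hooks, calling the parent logic and then ApplyPoisonDamage in each.
; ApplyPoisonDamage checks that the Character is valid, then passes EffectValue, truncated to an integer, to its GetDamage function.
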(fn ApplyPoisonDamage
  (bind _character (Variables|Default|GetCharacter))
  (Utilities|IsValid _character
    (:Is%20Valid
      (Default|GetDamage _character (Math|Float|Truncate (Variables|Default|GetEffectValue))))))

(fn FirstIteration
  (|CallParentFunction)
  (CallFunction|ApplyPoisonDamage))

(fn LastIteration
  (|CallParentFunction)
  (CallFunction|ApplyPoisonDamage))

(fn MiddleIteration
  (|CallParentFunction)
  (CallFunction|ApplyPoisonDamage))