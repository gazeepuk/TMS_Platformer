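; BP_EffectComponent is a component that keeps a list of effects, with functions to add, remove or clear them.
; AddEffect appends to the Effects array and prints the effect's display name, while RemoveEffect only takes the entry out of the array.
; ClearAllEffects calls RemoveEffect while looping over that same array, so elements can be skipped.
; The file shows no logic that applies or ticks the effects.
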(fn AddEffect
  (params (InEffect :type BP%20Effect%20Base%20Object%20Reference))
  (Utilities|Array|Add (Variables|Default|GetEffects) InEffect)
  (Development|PrintString (Utilities|String|Append "Added: " (Utilities|GetDisplayName InEffect))))

(fn ClearAllEffects
  (for _array_element (Variables|Default|GetEffects)
    (CallFunction|RemoveEffect _array_element)))

(fn RemoveEffect
  (params (InEffectToRemove :type BP%20Effect%20Base%20Object%20Reference))
  (Utilities|Array|RemoveItem (Variables|Default|GetEffects) InEffectToRemove))