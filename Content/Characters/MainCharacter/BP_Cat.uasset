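; BP_Cat is the cat main character, a child Blueprint that adds cat-specific animation and sound to inherited character actions.
; Damage, paralysis, death, healing, launch and landing overrides play montages, animations or sounds around their parent calls.
; Launch plays jump feedback only if CanJump passes after the parent call.
; Left mouse triggers an Attack montage and reuses the damage sound, with no hit logic here.
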(event EventBeginPlay
  (|CallParentFunction) ; This node is disabled and will not be called.\nDrag off pins to build functionality.
)

(event EventOnLanded
  (params (Hit :type Hit%20Result%20Structure%20%28by%20ref%29))
  (|CallParentFunction Hit)
  (Audio|PlaySoundatLocation "/Game/Sounds/Cat/SW_Land.SW_Land" (Transformation|GetActorLocation) "0, 0, 0" 1.0 1.0 0.0 0 0 0 0))

(event Input|MouseEvents|LeftMouseButton
  (params (Key :type Key%20Structure :default "None"))
  (:Pressed
    (CallFunction|Attack)
    (Audio|PlaySoundatLocation "/Game/Sounds/Cat/SC_CatGetDamage.SC_CatGetDamage" (Transformation|GetActorLocation) "0, 0, 0" 1.0 1.0 0.0 0 0 0 0)))

(fn ConstructionScript
  (|CallParentFunction))

(fn GetDamage
  (params (DamageValue :type Integer))
  (Animation|PlayAnimMontage "/Game/Characters/MainCharacter/Animations/AM_CatGetDamage.AM_CatGetDamage" 1.0 "None")
  (Audio|PlaySoundatLocation "/Game/Sounds/Cat/SC_CatGetDamage.SC_CatGetDamage" (Transformation|GetActorLocation) "0, 0, 0" 1.0 1.0 0.0 0 0 0 0)
  (|CallParentFunction DamageValue))

(fn Die
  (Components|Animation|PlayAnimation (Variables|Character|GetMesh) "/Game/Characters/MainCharacter/Animations/A_Cat-Die.A_Cat-Die" false)
  (|CallParentFunction))

(fn Paralize
  (Animation|PlayAnimMontage "/Game/Characters/MainCharacter/Animations/AM_Cat-Paralize.AM_Cat-Paralize" 1.0 "None")
  (Audio|PlaySoundatLocation "/Game/Sounds/Cat/SW_Zap.SW_Zap" (Transformation|GetActorLocation) "0, 0, 0" 1.0 1.0 0.0 0 0 0 0)
  (|CallParentFunction))

(fn Launch
  (|CallParentFunction)
  (if (Character|CanJump)
    (Animation|PlayAnimMontage "/Game/Characters/MainCharacter/Animations/AM_Cat-StartJump.AM_Cat-StartJump" 1.0 "None")
    (Audio|PlaySoundatLocation "/Game/Sounds/Cat/SW_Jump.SW_Jump" (Transformation|GetActorLocation) "0, 0, 0" 1.0 1.0 0.0 0 0 0 0)))

(fn Attack
  (Animation|PlayAnimMontage "/Game/Characters/MainCharacter/Animations/AM_Cat-Attack.AM_Cat-Attack" 1.0 "None"))

(fn Heal
  (params (HealValue :type Integer))
  (Audio|PlaySoundatLocation "/Game/Sounds/Cat/SC_Purring.SC_Purring" (Transformation|GetActorLocation) "0, 0, 0" 1.0 1.0 0.0 0 0 0 0)
  (|CallParentFunction HealValue))